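; BP_Character is a character Blueprint with health, melee attack and walk speed functions; its event graph and construction script are empty.
; IsAlive checks that Health is above zero, and UpdateWalkSpeed sets the movement component's maximum walk speed.
; DoMeleeAttack requires a living character with no montage playing, but currently only prints a debug string and sets the mesh's animation to Death_1, apparently as a placeholder.
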(event EventBeginPlay)

(event Collision|EventActorBeginOverlap
  (params (OtherActor :type Actor%20Object%20Reference)))

(event EventTick
  (params (DeltaSeconds :type Float%20%28single-precision%29)))

(fn ConstructionScript)

(fn IsAlive
  (return (> (Variables|Default|GetHealth) 0.0)))

(fn DoMeleeAttack
  (if (and (CallFunction|IsAlive) (not (Class|AnimInstance|IsAnyMontagePlaying (Components|SkeletalMesh|GetAnimInstance (Variables|Character|GetMesh)))))
    (Development|PrintString "Hello")
    (Components|Animation|SetAnimation (Variables|Character|GetMesh) "/Game/AnimStarterPack/Death_1.Death_1")))

(fn UpdateWalkSpeed
  (params (New%20Walk%20Speed :type Float%20%28single-precision%29))
  (Variables|/Script/Engine.CharacterMovementComponent|SetMaxWalkSpeed (Variables|Character|GetCharacterMovement) New%20Walk%20Speed))